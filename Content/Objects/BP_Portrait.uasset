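; BP_Portrait is a placeable portrait object that displays four configurable text labels.
; The construction script copies the Text1 to Text4 variables into four TextRender components, so the text updates when the instance is constructed.
; The event graph has no live logic, only an unconnected chain of SetVisibility calls that would show the text components.
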(event `self.ReceiveBeginPlay`)

(event `self.ReceiveTick`
  (params (DeltaSeconds :type "Float (single-precision)")))

(fn `UserConstructionScript`
  (`TextRenderComponent.K2_SetText` (`self.TextRender`) (`self.Text1`))
  (`TextRenderComponent.K2_SetText` (`self.TextRender1`) (`self.Text2`))
  (`TextRenderComponent.K2_SetText` (`self.TextRender2`) (`self.Text3`))
  (`TextRenderComponent.K2_SetText` (`self.TextRender3`) (`self.Text4`)))