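; Player pawn that restores its saved transform, counts clicks and interacts with radios.
; BeginPlay teleports the player to the location and rotation in MySaveGame's slot, which this file never writes.
; Left click increments and saves a click count, and line-traces from the camera to toggle actors implementing BP_RadioInterface.
; R deletes the save, 4 alternates playing a nursery rhyme with disabling input, and a LoadLevel teleport branch sits unconnected.
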(event `self.ReceiveBeginPlay`
  (bind _returnvalue (`GameplayStatics.LoadGameFromSlot` "Slot1"))
  (bind _output_get (set `self.SaverSubClass` _returnvalue))
  (bind _asmy_save_game (cast `/Game/StarterContent/Blueprints/MySaveGame` _output_get))
  (bind _actorlocation (`/Game/StarterContent/Blueprints/MySaveGame.ActorLocation` _asmy_save_game))
  (bind _actorrotation (`/Game/StarterContent/Blueprints/MySaveGame.ActorRotation` _asmy_save_game))
  (`self.K2_TeleportTo` (`GameplayStatics.GetPlayerPawn` 0) _actorlocation _actorrotation)
  (`KismetSystemLibrary.PrintString` (`KismetStringLibrary.Conv_VectorToString` _actorlocation))
  (`KismetSystemLibrary.PrintString` (`KismetStringLibrary.Conv_RotatorToString` _actorrotation)))

(event `Key|LeftMouseButton`
  (params (Key :type "Key Structure"))
  (bind _saversubclass (`self.SaverSubClass`))
  (:`Pressed`
    (bind _returnvalue (`GameplayStatics.DoesSaveGameExist` "Slot1"))
    (if _returnvalue
      (bind _returnvalue_2 (`GameplayStatics.LoadGameFromSlot` "Slot1"))
      (bind _output_get (set `self.SaverSubClass` _returnvalue_2))
      (bind _asmy_save_game (cast `/Game/StarterContent/Blueprints/MySaveGame` _output_get))
      (bind _result (`/Engine/EditorBlueprintResources/StandardMacros.IncrementInt` (`/Game/StarterContent/Blueprints/MySaveGame.NumOfClicks` _asmy_save_game))
        (:`  `
          (`GameplayStatics.SaveGameToSlot` _saversubclass "Slot1")
          (`KismetSystemLibrary.PrintString` (`KismetStringLibrary.Conv_IntToString` _result))))
      (else
        (bind _returnvalue_3 (`GameplayStatics.CreateSaveGameObject` "/Game/StarterContent/Blueprints/MySaveGame.MySaveGame_C"))
        (bind _output_get_2 (set `self.SaverSubClass` _returnvalue_3))
        (bind _asmy_save_game_2 (cast `/Game/StarterContent/Blueprints/MySaveGame` _output_get_2))
        (bind _result_2 (`/Engine/EditorBlueprintResources/StandardMacros.IncrementInt` (`/Game/StarterContent/Blueprints/MySaveGame.NumOfClicks` _asmy_save_game_2))
          (:`  `
            (`GameplayStatics.SaveGameToSlot` _saversubclass "Slot1")
            (`KismetSystemLibrary.PrintString` (`KismetStringLibrary.Conv_IntToString` _result_2))))))))

(event `Key|R`
  (params (Key :type "Key Structure"))
  (:`Pressed`
    (`GameplayStatics.DeleteGameInSlot` "Slot1")))

(event `Key|LeftMouseButton`
  (params (Key :type "Key Structure"))
  (:`Pressed`
    (`KismetSystemLibrary.PrintString` "Radio pressed")
    (bind _outhit (`self.Interact`))
    (bind (_bblockinghit _binitialoverlap _time _distance _location _impactpoint _normal _impactnormal _physmat _hitactor) (`GameplayStatics.BreakHitResult` _outhit))
    (if (`KismetSystemLibrary.DoesImplementInterface` _hitactor "/Game/StarterContent/Blueprints/BP_RadioInterface.BP_RadioInterface_C")
      (message `/Game/StarterContent/Blueprints/BP_RadioInterface.ToggleRadio` _hitactor))))

(event `Key|Four`
  (params (Key :type "Key Structure"))
  (:`Pressed`
    (`/Engine/EditorBlueprintResources/StandardMacros.FlipFlop`
      (:`A`
        (`GameplayStatics.PlaySoundAtLocation` "/Game/Audio/Mary_Had_a_Little_Lamb__Nursery_Rhyme__Kids_Songs_Animation_for_Children.Mary_Had_a_Little_Lamb__Nursery_Rhyme__Kids_Songs_Animation_for_Children" (352.0 -122.0 1000.0) (struct) 1.0 1.0 0.0 null null null))
      (:`B`
        (`self.DisableInput` null)))))

(fn `Interact`
  (returns (OutHit :type "HitResult Structure"))
  (bind _returnvalue (`GameplayStatics.GetPlayerCameraManager` 0))
  (bind _returnvalue_2 (`self.K2_GetActorLocation` _returnvalue))
  (bind _outhit (`KismetSystemLibrary.LineTraceSingle` _returnvalue_2 (+ _returnvalue_2 (* (`self.GetActorForwardVector` _returnvalue) 1000.0)) "TraceTypeQuery1"))
  (return _outhit))

(fn `UserConstructionScript`)