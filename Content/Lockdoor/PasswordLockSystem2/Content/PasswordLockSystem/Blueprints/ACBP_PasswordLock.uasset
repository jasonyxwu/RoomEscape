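; ACBP_PasswordLock is a Blueprint, likely an actor component, that adds a password lock which the player opens through a UI widget.
; UnlockEvent creates WB_Password_List with the password size, entered value and solution, switches to Game and UI input, disables character input and registers the widget on BP_PlayerController.
; Widget event bindings support clearing the Locked flag and copying the entered password back, so the component retains that state.
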(event `Unlock Event`
  (bind _returnvalue (`GameplayStatics.GetPlayerController` 0))
  ;[0 0 0] Unlock Event | Create Password List widget and display it, bind events, modify input mode and disable input for our character.
  (bind _returnvalue_2 (`|CreateWidget` "/Game/PasswordLockSystem/Blueprints/WB_Password_List.WB_Password_List_C" _returnvalue (`self.Password Size`) (`self.Password Entered`) (`self.Password to Unlock`)))
  (bind _output_get (set `self.Widget` _returnvalue_2))
  (`UserWidget.AddToViewport` _output_get 0)
  (add `/Game/PasswordLockSystem/Blueprints/WB_Password_List.Unlocked` _output_get (`|CreateDelegate` :!event `Modify bLocked`))
  (add `/Game/PasswordLockSystem/Blueprints/WB_Password_List.Update` _output_get (`|CreateDelegate` :!event `Modify Password`))
  (`WidgetBlueprintLibrary.SetInputMode_GameAndUIEx` _returnvalue _output_get)
  (`Actor.DisableInput` (`GameplayStatics.GetPlayerCharacter` 0) _returnvalue)
  (set `/Game/PasswordLockSystem/Blueprints/BP_PlayerController.Lock Widget` (`self.Widget`) (cast `/Game/PasswordLockSystem/Blueprints/BP_PlayerController` _returnvalue :!pure true)))

(event `Modify Password`
  ;[0 0 0] Modify Entered Password
  (set `self.Password Entered` (`/Game/PasswordLockSystem/Blueprints/WB_Password_List.Password Entered` (`self.Widget`))))

(event `Modify bLocked`
  ;[0 0 0] Modify bLocked
  (set `self.bLocked` false))