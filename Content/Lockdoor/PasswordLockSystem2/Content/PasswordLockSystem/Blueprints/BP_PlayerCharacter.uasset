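; First-person player character for a password lock system, handling movement, look and interaction, and creating the HUD on BeginPlay.
; Each tick, InteractableTrace casts a short camera ray, storing the hit and toggling custom depth to outline components tagged "Interactable".
; The Interact input sends InteractMessage to the traced actor if its component carries that tag.
; A gamepad face-left press only draws a debug trace.
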(event `self.ReceiveBeginPlay`
  (bind _returnvalue (`GameplayStatics.GetPlayerController` 0))
  ;[0 0 0] Create HUD widget and display it
  (bind _returnvalue_2 (`|CreateWidget` "/Game/PasswordLockSystem/Blueprints/WB_HUD.WB_HUD_C" _returnvalue))
  (bind _output_get (set `self.HUD` _returnvalue_2))
  (`UserWidget.AddToViewport` _output_get 0)
  (`WidgetBlueprintLibrary.SetInputMode_GameOnly` _returnvalue))

(event `self.ReceiveTick`
  (params (DeltaSeconds :type "Float (single-precision)"))
  ;[0 0 0] Trace for every frame
  (`self.Interactable Trace` 200.0))

(event `InputAxis|Move X`
  (params (AxisValue :type "Float (single-precision)"))
  ;[0 0 0] Movement Inputs
  (`self.AddMovementInput` (`self.GetActorRightVector`) AxisValue))

(event `InputAction|Interact`
  (params (Key :type "Key Structure"))
  (bind (_bblockinghit _binitialoverlap _time _distance _location _impactpoint _normal _impactnormal _physmat _hitactor _hitcomponent) (`GameplayStatics.BreakHitResult` (`self.Trace Hit`)))
  ;[0 0 0] Interact Inputs
  (:`Pressed`
    (`/Engine/EditorBlueprintResources/StandardMacros.IsValid` _hitcomponent
      (:`Is Valid`
        (if (`ActorComponent.ComponentHasTag` _hitcomponent "Interactable")
          (message `/Game/PasswordLockSystem/Blueprints/BPI_Interaction.Interact` _hitactor self))))))

(event `InputAxis|View X`
  (params (AxisValue :type "Float (single-precision)"))
  ;[0 0 0] View Inputs
  (`self.AddControllerYawInput` AxisValue))

(event `InputAxis|Move Y`
  (params (AxisValue :type "Float (single-precision)"))
  ;[0 0 0] Movement Inputs
  (`self.AddMovementInput` (`self.GetActorForwardVector`) AxisValue))

(event `InputAxis|View Y`
  (params (AxisValue :type "Float (single-precision)"))
  ;[0 0 0] View Inputs
  (`self.AddControllerPitchInput` AxisValue))

(event `Key|Gamepad_FaceButton_Left`
  (params (Key :type "Key Structure"))
  (bind _returnvalue (`GameplayStatics.GetPlayerCameraManager` 0))
  (bind _returnvalue_2 (`PlayerCameraManager.GetCameraLocation` _returnvalue))
  (:`Pressed`
    (`KismetSystemLibrary.LineTraceSingle` :`Start` _returnvalue_2 :`End` (+ _returnvalue_2 (* (`KismetMathLibrary.GetForwardVector` (`PlayerCameraManager.GetCameraRotation` _returnvalue)) 200.0)) :`TraceChannel` "TraceTypeQuery1" :`DrawDebugType` "ForDuration")))

(fn `Interactable Trace`
  (params (`Trace Distance` :type "Float (double-precision)" :default 200.0))
  (bind _returnvalue (`GameplayStatics.GetPlayerCameraManager` 0))
  (bind (_bblockinghit _binitialoverlap _time _distance _location _impactpoint _normal _impactnormal _physmat _hitactor _hitcomponent) (`GameplayStatics.BreakHitResult` (`self.Trace Hit`)))
  (bind _returnvalue_2 (`PlayerCameraManager.GetCameraLocation` _returnvalue))
  (`|ExecutionSequence`
    (:`then_0`
      ;[0 0 0] Reset Outline
      (`/Engine/EditorBlueprintResources/StandardMacros.IsValid` _hitcomponent
        (:`Is Valid`
          (`PrimitiveComponent.SetRenderCustomDepth` _hitcomponent false))))
    (:`then_1`
      ;[0 0 0] Line Trace for Interactable Objects and draw Outline
      (bind _outhit (`KismetSystemLibrary.LineTraceSingle` _returnvalue_2 (+ _returnvalue_2 (* (`KismetMathLibrary.GetForwardVector` (`PlayerCameraManager.GetCameraRotation` _returnvalue)) (`local.Trace Distance`))) "TraceTypeQuery1"))
      (bind _output_get (set `self.Trace Hit` _outhit))
      (bind (_bblockinghit_2 _binitialoverlap_2 _time_2 _distance_2 _location_2 _impactpoint_2 _normal_2 _impactnormal_2 _physmat_2 _hitactor_2 _hitcomponent_2) (`GameplayStatics.BreakHitResult` _output_get))
      (`/Engine/EditorBlueprintResources/StandardMacros.IsValid` _hitcomponent_2
        (:`Is Valid`
          (`PrimitiveComponent.SetRenderCustomDepth` _hitcomponent_2 (`ActorComponent.ComponentHasTag` _hitcomponent_2 "Interactable")))))))

(fn `UserConstructionScript`)