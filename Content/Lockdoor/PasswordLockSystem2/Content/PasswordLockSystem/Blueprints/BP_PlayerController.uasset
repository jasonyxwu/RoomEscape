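; Player controller for the password lock system that adds gamepad support to the lock UI.
; While LockWidget is in the viewport, Tick moves the mouse cursor from gamepad axis input scaled by Sensitivity, with vertical input inverted.
; Input actions forward click, cancel, increase and decrease presses to LockWidget whenever it is valid.
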(event `self.ReceiveTick`
  (params (DeltaSeconds :type "Float (single-precision)"))
  (bind (_locationx _locationy) (`self.GetMousePosition`))
  (bind _sensitivity (`self.Sensitivity`))
  ;[0 0 0] Gamepad Support - Simulate Mouse Movement
  (bind _lock_widget (`self.Lock Widget`)
    (:`then`
      (if (`Widget.IsInViewport` _lock_widget)
        (`self.SetMouseLocation` (`KismetMathLibrary.FTrunc` (+ (* (`self.GetInputAxisKeyValue`) _sensitivity) _locationx)) (`KismetMathLibrary.FTrunc` (+ (* (`self.GetInputAxisKeyValue`) _sensitivity -1.0) _locationy)))))
    (:`else`)))

(event `InputAction|SimulateClick`
  (params (Key :type "Key Structure"))
  ;[0 0 0] Gamepad Support - Simulate Click
  (:`Pressed`
    (bind _lock_widget (`self.Lock Widget`)
      (:`then`
        (`/Game/PasswordLockSystem/Blueprints/WB_Password_List.Simulate Click` _lock_widget))
      (:`else`))))

(event `InputAction|SimulateCancel`
  (params (Key :type "Key Structure"))
  ;[0 0 0] Gamepad Support - Simulate Cancel
  (:`Pressed`
    (bind _lock_widget (`self.Lock Widget`)
      (:`then`
        (`/Game/PasswordLockSystem/Blueprints/WB_Password_List.Cancel` _lock_widget))
      (:`else`))))

(event `InputAction|SimulateIncrease`
  (params (Key :type "Key Structure"))
  ;[0 0 0] Gamepad Support - Simulate Increase
  (:`Pressed`
    (bind _lock_widget (`self.Lock Widget`)
      (:`then`
        (`/Game/PasswordLockSystem/Blueprints/WB_Password_List.Simulate Increase` _lock_widget))
      (:`else`))))

(event `InputAction|SimulateDecrease`
  (params (Key :type "Key Structure"))
  ;[0 0 0] Gamepad Support - Simulate Decrease
  (:`Pressed`
    (bind _lock_widget (`self.Lock Widget`)
      (:`then`
        (`/Game/PasswordLockSystem/Blueprints/WB_Password_List.Simulate Decrease` _lock_widget))
      (:`else`))))

(fn `UserConstructionScript`)