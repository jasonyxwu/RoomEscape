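; BP_ExampleDoor is an example interactable door for the password lock system.
; On Interact, it asks its password lock component to start unlocking if locked, otherwise toggles between open and closed.
; A single timeline drives the door mesh's yaw, playing forward to open and reversing to close, with a sound cue for each direction.
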(event `/Game/PasswordLockSystem/Blueprints/BPI_Interaction.Interact`
  (params (Character :type "Character Object Reference"))
  ;[0 0 0] Blueprint Interface
  ;[0 0 0] If the door is locked, then start trying to unlock.
  (`self.Locked?`
    (:`true`
      (`/Game/PasswordLockSystem/Blueprints/ACBP_PasswordLock.Unlock Event` (`self.ACBP_PasswordLock`)))
    (:`false`
      ;[0 0 0] If the door is not locked, then open or close the door.
      (`self.Opened?`
        (:`Ture`
          (`self.Door Close`))
        (:`False`
          (`self.Door Open`))))))

(event `Door Open`
  ;[0 0 0] Open the door
  (set `self.Door Opened` true)
  (`GameplayStatics.PlaySoundAtLocation` "/Game/PasswordLockSystem/Audio/Cue_DoorOpen.Cue_DoorOpen" (`self.K2_GetActorLocation`) (struct) 1.0 1.0 0.0 null null null)
  ;[0 0 0] Timeline for Open/Close door animation
  (bind (_direction _movement) (`Timeline|Timeline` :!label _label)
    (:`Update`
      (`SceneComponent.K2_SetRelativeRotation` (`self.SM_Door`) (`KismetMathLibrary.MakeRotator` 0.0 0.0 _movement) false false))))

(event `Door Close`
  ;[0 0 0] Close the door
  (set `self.Door Opened` false)
  (`GameplayStatics.PlaySoundAtLocation` "/Game/PasswordLockSystem/Audio/Cue_DoorClose.Cue_DoorClose" (`self.K2_GetActorLocation`) (struct) 1.0 1.0 0.0 null null null)
  (goto _label :!via `Reverse`))

(fn `UserConstructionScript`)