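; Room-escape trigger actor that shows the SolutionPuzzle widget when the FirstPersonCharacter overlap count across its four boxes reaches four.
; Each box increments a shared Count on begin overlap and decrements it on end overlap.
; Tick polls that count, rechecks it after a short delay, then displays the widget created at BeginPlay for a few seconds, with a Showing flag preventing repeat displays meanwhile.
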(event `self.ReceiveBeginPlay`
  (bind _returnvalue (`|CreateWidget` "/Game/RoomEscape/UI/SolutionPuzzle.SolutionPuzzle_C"))
  (set `self.UI` _returnvalue))

(event `self.ReceiveTick`
  (params (DeltaSeconds :type "Float (single-precision)"))
  (bind _ui (`self.UI`))
  (if (== (`self.Count`) 4)
    (if (not (`self.Showing`))
      (`KismetSystemLibrary.Delay` 0.2)
      (if (== (`self.Count`) 4)
        (set `self.Showing` true)
        (`UserWidget.AddToViewport` _ui 0)
        (`KismetSystemLibrary.Delay` 5.0)
        (`Widget.RemoveFromParent` _ui)
        (set `self.Showing` false)))))

(event `self.Box.OnComponentBeginOverlap`
  (params (OverlappedComponent :type "PrimitiveComponent Object Reference") (OtherActor :type "Actor Object Reference") (OtherComp :type "PrimitiveComponent Object Reference") (OtherBodyIndex :type Integer) (bFromSweep :type Boolean) (SweepResult :type "HitResult Structure (by ref)"))
  (cast `/Game/RoomEscape/Blueprints/FirstPersonCharacter` OtherActor)
  (set `self.Count` (+ (`self.Count`) 1)))

(event `self.Box.OnComponentEndOverlap`
  (params (OverlappedComponent :type "PrimitiveComponent Object Reference") (OtherActor :type "Actor Object Reference") (OtherComp :type "PrimitiveComponent Object Reference") (OtherBodyIndex :type Integer))
  (cast `/Game/RoomEscape/Blueprints/FirstPersonCharacter` OtherActor)
  (set `self.Count` (- (`self.Count`) 1)))

(event `self.Box1.OnComponentBeginOverlap`
  (params (OverlappedComponent :type "PrimitiveComponent Object Reference") (OtherActor :type "Actor Object Reference") (OtherComp :type "PrimitiveComponent Object Reference") (OtherBodyIndex :type Integer) (bFromSweep :type Boolean) (SweepResult :type "HitResult Structure (by ref)"))
  (cast `/Game/RoomEscape/Blueprints/FirstPersonCharacter` OtherActor)
  (set `self.Count` (+ (`self.Count`) 1)))

(event `self.Box1.OnComponentEndOverlap`
  (params (OverlappedComponent :type "PrimitiveComponent Object Reference") (OtherActor :type "Actor Object Reference") (OtherComp :type "PrimitiveComponent Object Reference") (OtherBodyIndex :type Integer))
  (cast `/Game/RoomEscape/Blueprints/FirstPersonCharacter` OtherActor)
  (set `self.Count` (- (`self.Count`) 1)))

(event `self.Box2.OnComponentBeginOverlap`
  (params (OverlappedComponent :type "PrimitiveComponent Object Reference") (OtherActor :type "Actor Object Reference") (OtherComp :type "PrimitiveComponent Object Reference") (OtherBodyIndex :type Integer) (bFromSweep :type Boolean) (SweepResult :type "HitResult Structure (by ref)"))
  (cast `/Game/RoomEscape/Blueprints/FirstPersonCharacter` OtherActor)
  (set `self.Count` (+ (`self.Count`) 1)))

(event `self.Box2.OnComponentEndOverlap`
  (params (OverlappedComponent :type "PrimitiveComponent Object Reference") (OtherActor :type "Actor Object Reference") (OtherComp :type "PrimitiveComponent Object Reference") (OtherBodyIndex :type Integer))
  (cast `/Game/RoomEscape/Blueprints/FirstPersonCharacter` OtherActor)
  (set `self.Count` (- (`self.Count`) 1)))

(event `self.Box3.OnComponentBeginOverlap`
  (params (OverlappedComponent :type "PrimitiveComponent Object Reference") (OtherActor :type "Actor Object Reference") (OtherComp :type "PrimitiveComponent Object Reference") (OtherBodyIndex :type Integer) (bFromSweep :type Boolean) (SweepResult :type "HitResult Structure (by ref)"))
  (cast `/Game/RoomEscape/Blueprints/FirstPersonCharacter` OtherActor)
  (set `self.Count` (+ (`self.Count`) 1)))

(event `self.Box3.OnComponentEndOverlap`
  (params (OverlappedComponent :type "PrimitiveComponent Object Reference") (OtherActor :type "Actor Object Reference") (OtherComp :type "PrimitiveComponent Object Reference") (OtherBodyIndex :type Integer))
  (cast `/Game/RoomEscape/Blueprints/FirstPersonCharacter` OtherActor)
  (set `self.Count` (- (`self.Count`) 1)))

(fn `UserConstructionScript`)